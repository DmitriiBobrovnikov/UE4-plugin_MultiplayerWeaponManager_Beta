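; Player character Blueprint that handles movement, camera look and weapon input.
; Movement axes follow control yaw only, while look axes drive controller yaw and pitch.
; Weapon logic is delegated to GameWeaponManager: number keys 1–3 all create BP_FireWeapon, and key 4 passes no class, noted as destroying the weapon.
; Fire and Aim press/release start and stop the weapon's primary and special actions.
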(event Input|ActionEvents|InputActionFire
  (params (Key :type Key%20Structure :default "None"))
  (bind _gameweaponmanager (Variables|Default|GetGameWeaponManager))
  ;[0.02275 1 0] UseWeapon
  ;;[0 0.6756 1] Use Weapon (Use Weapon Attack) Left mouse button
  (:Pressed
    (Class|GameWeaponManager|Fire _gameweaponmanager))
  (:Released
    (Class|GameWeaponManager|StopFire _gameweaponmanager)))

(event Input|ActionEvents|InputActionAim
  (params (Key :type Key%20Structure :default "None"))
  (bind _gameweaponmanager (Variables|Default|GetGameWeaponManager))
  ;[0.02275 1 0] UseWeapon
  ;;[0 0.6659 1] UseSpecifical Action (Attac or Aim or ... ) Right mouseButton
  (:Pressed
    (Class|GameWeaponManager|Specific _gameweaponmanager))
  (:Released
    (Class|GameWeaponManager|StopSpecific _gameweaponmanager)))

(event Input|AxisEvents|InputAxisMoveForward
  (params (AxisValue :type Float%20%28single-precision%29))
  ;[1 1 1] Movement
  ;;[1 0.9582 0] Character controlle
  (Pawn|Input|AddMovementInput (Math|Vector|GetForwardVector (Math|Rotator|MakeRotator 0.0 0.0 (.yaw (Pawn|GetControlRotation :!class /Script/Engine.Pawn)))) AxisValue false))

(event Input|AxisEvents|InputAxisMoveRight
  (params (AxisValue :type Float%20%28single-precision%29))
  ;[1 1 1] Movement
  ;;[1 0.9582 0] Character controlle
  (Pawn|Input|AddMovementInput (Math|Vector|GetRightVector (Math|Rotator|MakeRotator 0.0 0.0 (.yaw (Pawn|GetControlRotation :!class /Script/Engine.Pawn)))) AxisValue false))

(event Input|AxisEvents|InputAxisTurn
  (params (AxisValue :type Float%20%28single-precision%29))
  ;[1 1 1] Movement
  ;;[1 0.8839 0] Camera controll
  (Pawn|Input|AddControllerYawInput AxisValue))

(event Input|AxisEvents|InputAxisLookUp
  (params (AxisValue :type Float%20%28single-precision%29))
  ;[1 1 1] Movement
  ;;[1 0.8839 0] Camera controll
  (Pawn|Input|AddControllerPitchInput AxisValue))

(event Input|KeyboardEvents|1
  (params (Key :type Key%20Structure :default "None"))
  ;[1 0 0] Create Weapon (Is Weapon class != null result create weapon  or Weapon class == Null result Destroy weapon)
  (:Pressed
    (Class|GameWeaponManager|CreateWeapon (Variables|Default|GetGameWeaponManager) "/WeaponManager/Blueprint/Weapon/BP_FireWeapon.BP_FireWeapon_C")))

(event Input|KeyboardEvents|4
  (params (Key :type Key%20Structure :default "None"))
  ;[1 0 0] Create Weapon (Is Weapon class != null result create weapon  or Weapon class == Null result Destroy weapon)
  (:Pressed
    (Class|GameWeaponManager|CreateWeapon (Variables|Default|GetGameWeaponManager))))

(event Input|KeyboardEvents|2
  (params (Key :type Key%20Structure :default "None"))
  ;[1 0 0] Create Weapon (Is Weapon class != null result create weapon  or Weapon class == Null result Destroy weapon)
  (:Pressed
    (Class|GameWeaponManager|CreateWeapon (Variables|Default|GetGameWeaponManager) "/WeaponManager/Blueprint/Weapon/BP_FireWeapon.BP_FireWeapon_C")))

(event Input|KeyboardEvents|3
  (params (Key :type Key%20Structure :default "None"))
  ;[1 0 0] Create Weapon (Is Weapon class != null result create weapon  or Weapon class == Null result Destroy weapon)
  (:Pressed
    (Class|GameWeaponManager|CreateWeapon (Variables|Default|GetGameWeaponManager) "/WeaponManager/Blueprint/Weapon/BP_FireWeapon.BP_FireWeapon_C")))

(fn ConstructionScript)